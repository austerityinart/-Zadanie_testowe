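; BP_BOT2 is a bot that uses AIMoveTo to travel to an actor from its Target array.
; BeginPlay increments an index and, only when it exceeds the last array index, resets it to zero and starts the move; otherwise nothing follows.
; Success or failure both lead to a three-second delay, then the Onmove event re-enters the same increment-and-check logic.
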(event `self.ReceiveBeginPlay`
  ; 1
  (`/Engine/EditorBlueprintResources/StandardMacros.IncrementInt` (`self.int`) :!label _label
    (:`  `
      (if (> (`self.int`) (`KismetArrayLibrary.Array_LastIndex` (`self.Target`)))
        (set `self.int` 0)
        (`|AIMoveTo` self (0.0 0.0 0.0) (`|GetArrayItem` (`self.Target`) (`self.int`))
          (:`OnSuccess`
            _)
          (:`OnFail`
            _))
        (`KismetSystemLibrary.Delay` 3.0)
        (`self.Onmove`)))))

(event `Onmove`
  ; 1
  (goto _label))

(fn `UserConstructionScript`)